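; BP_Cube_OSC is a cube actor controlled over OSC through EMDMOSC nodes, which also reports touches back.
; Incoming messages on rotation addresses drive one shared relative-rotation setter, summing the single X value with the vector's X.
; Color messages create a dynamic M_Cube material instance and set its Color.
; Actor hits send the impact location as a string to /cube/touched; the similar click handler is never bound.
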(event `OnActorHit_Event` :!signature `self.OnActorHit`
  (params (SelfActor :type "Actor Object Reference") (OtherActor :type "Actor Object Reference") (NormalImpulse :type "Vector Structure") (Hit :type "HitResult Structure (by ref)"))
  (`/Game/Blueprints/EMDM-OSC-Interface.EMDM_OSC_Out` "/cube/touched" "String" false 0 0.0 (`KismetStringLibrary.Conv_VectorToString` (`.Location` (`GameplayStatics.BreakHitResult` Hit))) (`|MakeArray` 0.0) :!label _label) ; Need to get the Target to address all actors...
)

(event `OnClicked_Event` :!signature `self.OnClicked`
  (params (TouchedActor :type "Actor Object Reference") (ButtonPressed :type "Key Structure" :default "None"))
  (goto _label))

(event `self.ReceiveBeginPlay`
  (add `self.OnActorHit` (delegate `OnActorHit_Event`))
  (`GameplayStatics.GetAllActorsWithInterface` "/Game/Blueprints/EMDM-OSC-Interface.EMDM-OSC-Interface_C"))

(event `/Game/Blueprints/EMDM-OSC-Interface.EMDM OSC In`
  (params (OSC_Message :type "OSCMessage Structure"))
  (`|ExecutionSequence`
    (:`then_0`
      (bind _float (`/Game/Blueprints/EMDM-OSC-Macro-Library.EMDM_OSC_Float` "/cube/rotation/x" OSC_Message 0.0 360.0)
        (:`Received`
          (bind (_x _y _z) (`KismetMathLibrary.BreakVector3f` (stale _vec3f)))
          (`SceneComponent.K2_SetRelativeRotation` (`self.StaticMeshComponent`) (`KismetMathLibrary.MakeRotator` (+ _float _x) _y _z) false false :!label _label_2))))
    (:`then_1`
      (bind _vec3f (`/Game/Blueprints/EMDM-OSC-Macro-Library.EMDM_OSC_Floats_to_Vec3f` "/cube/rotation" OSC_Message 0.0 360.0)
        (:`Received`
          (goto _label_2))))
    (:`then_2`
      (bind _color (`/Game/Blueprints/EMDM-OSC-Macro-Library.EMDM_OSC_Floats_to_Color` "/cube/color" OSC_Message)
        (:`Received`
          (bind _returnvalue (`PrimitiveComponent.CreateDynamicMaterialInstance` (`self.StaticMeshComponent`) 0 "/Game/M_Cube.M_Cube" "None"))
          (`MaterialInstanceDynamic.SetVectorParameterValue` _returnvalue "Color" _color))))))

(fn `UserConstructionScript`)